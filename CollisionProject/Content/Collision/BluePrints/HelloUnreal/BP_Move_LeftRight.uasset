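; BP_Move_LeftRight is an actor that slides its static mesh back and forth along its relative X axis.
; The Play event starts a timeline whose value, scaled to a distance, sets the mesh's relative location.
; When the timeline finishes, IsMoveRight flips and execution loops back to play or reverse it, producing continuous ping-pong motion.
; An EnableInput call for the first player controller is left unconnected.
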(event Custom|Play
  (if (Variables|Default|GetIsMoveRight) :!label _label
    (bind _value (Timeline|타임라인_0 Play)
      (:Update
        (Transformation|SetRelativeLocation (Variables|Default|GetStaticMesh) (Math|Vector|MakeVector (* _value 1e+03) 0.0 0.0) false false))
      (:Finished
        (Variables|Default|SetIsMoveRight (not (Variables|Default|GetIsMoveRight)))
        (goto _label)))
    (else
      (Timeline|타임라인_0 Reverse))))

(fn ConstructionScript)